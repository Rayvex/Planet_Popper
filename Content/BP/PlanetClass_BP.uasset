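; Planet Blueprint for a game where the player spins a sphere and shoots pimples that spawn on it.
; While the rotate input is held, Tick adds axis input to the sphere's rotation and advances the spawn timer.
; Each spawn attaches a Pimple_BP at a random direction at planet radius, then scales the next interval.
; A debug-drawn camera-forward trace runs every tick, destroying hit "Kill"-tagged actors after shoot input.
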(event Custom|Destroy%20Pimples
  (bind _camera (Variables|Default|GetCamera))
  (bind _returnvalue (Transformation|GetWorldLocation _camera))
  ;[1 0 0.01123] Destroy Pimples
  (bind _outhit (Collision|LineTraceByChannel _returnvalue (+ _returnvalue (* (Math|Vector|GetForwardVector (Transformation|GetWorldRotation _camera)) (Variables|Default|GetLineLenght))) "TraceTypeQuery1" false 0 "Persistent" false))
  (if (Variables|Default|GetAttack)
    (if (Actor|ActorHasTag (.HitActor (Collision|BreakHitResult _outhit)) "Kill")
      (Actor|DestroyActor (.HitActor (Collision|BreakHitResult _outhit)))
      (else
        (Variables|Default|SetAttack false :!label _label)))
    (else
      (goto _label))))

(event Custom|Spawn%20Pimples
  (bind _sphere (Variables|Default|GetSphere))
  (bind _returnvalue (Transformation|GetWorldLocation _sphere))
  ;[0 0.07094 1] Spawn Pimples randomly on the planet
  (bind _outhit (Collision|LineTraceByChannel (Math|Vector|MakeVector (.x _returnvalue) (.y _returnvalue) (.z _returnvalue)) (+ (* (Math|Vector|GetForwardVector (Math|Rotator|MakeRotator (Math|Random|RandomFloatinRange (Variables|Default|GetMinRotation) (Variables|Default|GetMaxRotation)) (Math|Random|RandomFloatinRange (Variables|Default|GetMinRotation) (Variables|Default|GetMaxRotation)) (Math|Random|RandomFloatinRange (Variables|Default|GetMinRotation) (Variables|Default|GetMaxRotation)))) (Variables|Default|GetPlanetRadius)) (Transformation|GetWorldLocation (Variables|Default|GetSphere))) "TraceTypeQuery1" false 0 "None" false))
  (bind _returnvalue_2 (Game|SpawnActorfromClass "/Game/BP/Pimple_BP.Pimple_BP_C" (Math|Transform|MakeTransform (.traceend _outhit) "0, 0, 0" "1,1,1") "Undefined" 0 0))
  (Transformation|AttachComponentToComponent _returnvalue_2 (Variables|Default|GetSphere) "None" "KeepWorld" "KeepRelative" "KeepRelative" true)
  (Variables|Default|SetTime 0.0)
  (Variables|Default|SetSpawnSpeed (* (Variables|Default|GetSpawnSpeed) (Variables|Default|GetSpawnSpeedChange))))

(event Custom|RotateWorld
  ;[1 0 0.5973] WorldRotation
  (Transformation|SetWorldRotation (Variables|Default|GetSphere) (Math|Rotator|MakeRotator (.x (+ (Math|Vector|MakeVector (.roll (Variables|Default|GetNextRotation)) (.pitch (Variables|Default|GetNextRotation)) (.yaw (Variables|Default|GetNextRotation))) (Math|Vector|MakeVector (Class|Actor|GetInputAxisKeyValue) (Class|Actor|GetInputAxisKeyValue) 0.0))) (.y (+ (Math|Vector|MakeVector (.roll (Variables|Default|GetNextRotation)) (.pitch (Variables|Default|GetNextRotation)) (.yaw (Variables|Default|GetNextRotation))) (Math|Vector|MakeVector (Class|Actor|GetInputAxisKeyValue) (Class|Actor|GetInputAxisKeyValue) 0.0))) (.z (+ (Math|Vector|MakeVector (.roll (Variables|Default|GetNextRotation)) (.pitch (Variables|Default|GetNextRotation)) (.yaw (Variables|Default|GetNextRotation))) (Math|Vector|MakeVector (Class|Actor|GetInputAxisKeyValue) (Class|Actor|GetInputAxisKeyValue) 0.0)))) false false)
  (Variables|Default|SetNextRotation (Math|Rotator|MakeRotator (.x (+ (Math|Vector|MakeVector (.roll (Variables|Default|GetNextRotation)) (.pitch (Variables|Default|GetNextRotation)) (.yaw (Variables|Default|GetNextRotation))) (Math|Vector|MakeVector (Class|Actor|GetInputAxisKeyValue) (Class|Actor|GetInputAxisKeyValue) 0.0))) (.y (+ (Math|Vector|MakeVector (.roll (Variables|Default|GetNextRotation)) (.pitch (Variables|Default|GetNextRotation)) (.yaw (Variables|Default|GetNextRotation))) (Math|Vector|MakeVector (Class|Actor|GetInputAxisKeyValue) (Class|Actor|GetInputAxisKeyValue) 0.0))) 0.0)))

(event EventTick
  (params (DeltaSeconds :type Float%20%28single-precision%29))
  ;[0.326 0 1] Tick
  (if true
    (CallFunction|DestroyPimples)
    (if (Variables|Default|GetRMDown)
      (CallFunction|RotateWorld)
      (if (> (Variables|Default|GetTime) (Variables|Default|GetSpawnSpeed))
        (CallFunction|SpawnPimples))
      (Variables|Default|SetTime (+ (Variables|Default|GetTime) (Variables|Default|GetTimeTick))))))

(event Input|ActionEvents|InputActionRotate_World
  (params (Key :type Key%20Structure :default "None"))
  ;[1 0 0.5973] WorldRotation
  (:Pressed
    (Variables|Default|SetRMDown true))
  (:Released
    (Variables|Default|SetRMDown false)))

(event Input|ActionEvents|InputActionShoot_World
  (params (Key :type Key%20Structure :default "None"))
  (:Pressed
    (Variables|Default|SetAttack true)))

(fn ConstructionScript)